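; BP_MapController is a pawn that provides player camera control over the map, with movement, rotation and zoom.
; Enhanced Input actions drive planar movement input along control-rotation axes and add relative yaw to the spring arm.
; Zoom input blends with the previous rate through a delta-time Lerp, then adjusts the spring arm length within clamped limits.
; Movement follows control rotation, independent of the spring arm's relative yaw.
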(event `self.ReceiveTick`
  (params (DeltaSeconds :type "Float (single-precision)")))

(event `EnhancedInput|/Game/WarOfNanite/Input/IA_Zoom`
  (params (ActionValue :type "Float (double-precision)") (ElapsedSeconds :type "Float (double-precision)") (TriggeredSeconds :type "Float (double-precision)") (InputAction :type "InputAction Object Reference" :default "/Game/WarOfNanite/Input/IA_Zoom.IA_Zoom"))
  (bind _springarm1 (`self.SpringArm1`))
  ; CameraZoom
  (:`Triggered`
    (bind _output_get (set `self.Zoomrate` (`KismetMathLibrary.Lerp` (* ActionValue 100.0) (`self.Zoomrate`) (* (`GameplayStatics.GetWorldDeltaSeconds`) 10.0))))
    (set `SpringArmComponent.TargetArmLength` (`KismetMathLibrary.FClamp` (+ (`SpringArmComponent.TargetArmLength` _springarm1) _output_get) 500.0 10000.0) _springarm1)))

(event `EnhancedInput|/Game/WarOfNanite/Input/IA_CamRotation`
  (params (ActionValue :type "Float (double-precision)") (ElapsedSeconds :type "Float (double-precision)") (TriggeredSeconds :type "Float (double-precision)") (InputAction :type "InputAction Object Reference" :default "/Game/WarOfNanite/Input/IA_CamRotation.IA_CamRotation"))
  ; Rotation
  (:`Triggered`
    (`SceneComponent.K2_AddRelativeRotation` (`self.SpringArm1`) (`KismetMathLibrary.MakeRotator` 0.0 0.0 ActionValue) false false)))

(event `EnhancedInput|/Game/WarOfNanite/Input/IA_CamMovement`
  (params (ActionValue :type "Vector2D Structure") (ElapsedSeconds :type "Float (double-precision)") (TriggeredSeconds :type "Float (double-precision)") (InputAction :type "InputAction Object Reference" :default "/Game/WarOfNanite/Input/IA_CamMovement.IA_CamMovement"))
  (bind (_returnvalue_roll _returnvalue_pitch _returnvalue_yaw) (`KismetMathLibrary.BreakRotator` (`self.GetControlRotation`)))
  (bind (_returnvalue_roll_2 _returnvalue_pitch_2 _returnvalue_yaw_2) (`KismetMathLibrary.BreakRotator` (`self.GetControlRotation`)))
  ; CameraMovement
  (:`Triggered`
    (`self.AddMovementInput` (`KismetMathLibrary.GetRightVector` (`KismetMathLibrary.MakeRotator` _returnvalue_roll_2 0.0 _returnvalue_yaw_2)) ActionValue_X)
    (`self.AddMovementInput` (`KismetMathLibrary.GetForwardVector` (`KismetMathLibrary.MakeRotator` 0.0 0.0 _returnvalue_yaw)) ActionValue_Y)))

(fn `UserConstructionScript`)